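; TPS player Blueprint in a retargeting sample that connects the character to its screen UI.
; BeginPlay creates the UI_Screen widget, then after a short delay fills in the HP ratio and text and resets the weapon display to non-grenade.
; OnUsingGrenade passes the grenade flag to that widget and triggers its weapon swap.
; OnGameOver calls the parent, shows the mouse cursor and adds the game-over widget.
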(event `self.OnGameOver`
  (bind _returnvalue (`GameplayStatics.GetPlayerController` 0))
  (`parent.OnGameOver`)
  (set `PlayerController.bShowMouseCursor` true _returnvalue)
  (bind _returnvalue_2 (`|CreateWidget` "/Game/3-3-7-UI/UI_GameOver.UI_GameOver_C" _returnvalue))
  (`UserWidget.AddToViewport` _returnvalue_2 0))

(event `self.ReceiveBeginPlay`
  (bind _returnvalue (`|CreateWidget` "/Game/3-3-7-UI/UI_Screen.UI_Screen_C" (`GameplayStatics.GetPlayerController` 0)))
  (set `self.uiScreen` _returnvalue)
  (`UserWidget.AddToViewport` (`self.uiScreen`) 0)
  (`KismetSystemLibrary.Delay` 0.05)
  (`self.UIctrl HP`)
  (`self.OnUsingGrenade` false))

(event `self.ReceiveTick`
  (params (DeltaSeconds :type "Float (single-precision)")))

(event `self.OnUsingGrenade`
  (params (isGrenade :type Boolean))
  (bind _uiscreen (`self.uiScreen`))
  (`/Engine/EditorBlueprintResources/StandardMacros.IsValid` _uiscreen
    (:`Is Valid`
      (set `/Game/3-3-7-UI/UI_Screen.isGrenaded` isGrenade _uiscreen)
      (`/Game/3-3-7-UI/UI_Screen.SwapWeapon` _uiscreen))))

(fn `UIctrl HP`
  (set `/Game/3-3-7-UI/UI_Screen.hpRatio` (/ (`KismetMathLibrary.Conv_IntToDouble` (`self.hp`)) (`KismetMathLibrary.Conv_IntToDouble` (`self.initialHp`))) (`self.uiScreen`))
  (set `/Game/3-3-7-UI/UI_Screen.hpString` (`KismetStringLibrary.Concat_StrStr` (`KismetStringLibrary.Conv_IntToString` (`self.hp`)) "/" (`KismetStringLibrary.Conv_IntToString` (`self.initialHp`))) (`self.uiScreen`)))

(fn `UserConstructionScript`)